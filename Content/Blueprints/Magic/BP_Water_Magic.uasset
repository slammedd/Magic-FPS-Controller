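; BP_Water_Magic is the water spell that spawns a BP_Water_Bubble in front of the player's view.
; StartCasting plays a bubble sound at its own location, then spawns the bubble at SpawnDistance along the camera's forward vector, using the player capsule's rotation.
; A Casting flag and a CastCooldown delay block recasting until the cooldown ends.
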(event EventStartCasting
  (bind _returnvalue (Game|GetPlayerCameraManager 0))
  (bind _transformcomponent (Variables|/Script/Engine.PlayerCameraManager|GetTransformComponent _returnvalue))
  (if (not (Variables|Default|GetCasting))
    (Variables|Default|SetCasting true)
    (Audio|PlaySoundatLocation "/Game/Audio/SC_Bubble_Spawn.SC_Bubble_Spawn" (Transformation|GetActorLocation) "0, 0, 0" 1.0 1.0 0.0 0 0 0 0)
    (Game|SpawnActorfromClass "/Game/Blueprints/Magic/BP_Water_Bubble.BP_Water_Bubble_C" (Math|Transform|MakeTransform (+ (* (Math|Vector|GetForwardVector _transformcomponent) (Variables|Default|GetSpawn%20Distance)) (Transformation|GetWorldLocation _transformcomponent)) (Transformation|GetWorldRotation (Variables|/Script/Engine.Character|GetCapsuleComponent (Game|GetPlayerCharacter 0))) "1.000000,1.000000,1.000000") "AdjustIfPossibleButAlwaysSpawn" "MultiplyWithRoot" 0 0)
    (Utilities|FlowControl|Delay (Variables|Default|GetCast%20Cooldown))
    (Variables|Default|SetCasting false)))

(fn ConstructionScript
  (|CallParentFunction))