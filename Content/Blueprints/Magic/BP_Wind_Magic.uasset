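; Wind magic spell for the first-person player that pushes enemies and ground pieces while casting.
; Start and stop casting toggle the VFX, fade the cast sound on the player's audio component, and set the Casting flag.
; Each tick while casting, a camera line trace launches imps with an impact effect, or drops ground pieces and adds an impulse.
; Push direction and force come from the player-to-impact vector scaled by WindStrength.
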(event EventStartCasting
  (bind _asbp_first_person_character (Utilities|Casting|CastToBP_FirstPersonCharacter (Game|GetPlayerCharacter 0)))
  (Audio|Components|Audio|SetSound (Variables|/Game/Blueprints/BP_FirstPersonCharacter.BP_FirstPersonCharacter_C|GetAudio%20Component _asbp_first_person_character) (Variables|Default|GetCast%20Sound))
  (Audio|Components|Audio|FadeIn (Variables|/Game/Blueprints/BP_FirstPersonCharacter.BP_FirstPersonCharacter_C|GetAudio%20Component _asbp_first_person_character) 1.0 1.0 0.0 "Linear" :!class /Script/Engine.AudioComponent)
  (Components|Activation|Activate (Variables|Default|GetMagic%20VFX) false)
  (Variables|Default|SetCasting true))

(event EventStopCasting
  (Components|Activation|Deactivate (Variables|Default|GetMagic%20VFX))
  (bind _asbp_first_person_character (Utilities|Casting|CastToBP_FirstPersonCharacter (Game|GetPlayerCharacter 0)))
  (Audio|Components|Audio|FadeOut (Variables|/Game/Blueprints/BP_FirstPersonCharacter.BP_FirstPersonCharacter_C|GetAudio%20Component _asbp_first_person_character) 1.0 0.0 "Linear" :!class /Script/Engine.AudioComponent)
  (Variables|Default|SetCasting false))

(event EventTick
  (params (DeltaSeconds :type Float%20%28single-precision%29))
  (bind _returnvalue (Game|GetPlayerCameraManager 0))
  (bind _transformcomponent (Variables|/Script/Engine.PlayerCameraManager|GetTransformComponent _returnvalue))
  (bind _returnvalue_2 (Math|Vector|GetForwardVector _transformcomponent))
  (bind _returnvalue_3 (Transformation|GetWorldLocation _transformcomponent))
  (bind _returnvalue_4 (+ _returnvalue_3 _returnvalue_2))
  (if (Variables|Default|GetCasting)
    (bind (_outhit _returnvalue_5) (Collision|LineTraceByChannel _returnvalue_4 (+ _returnvalue_4 (* _returnvalue_2 (Variables|Default|GetCast%20Distance))) "TraceTypeQuery1" false 0 "None"))
    (if _returnvalue_5
      (if (Utilities|DoesObjectImplementInterface (.HitActor (Collision|BreakHitResult _outhit)) "/Game/Blueprints/BPI_Enemy.BPI_Enemy_C")
        (bind _asbp_imp (Utilities|Casting|CastToBP_Imp (.HitActor (Collision|BreakHitResult _outhit))))
        (Niagara|SpawnSystematLocation "/Game/VFX/NS_Wind_Impact.NS_Wind_Impact" (.ImpactPoint (Collision|BreakHitResult _outhit)))
        (Character|LaunchCharacter _asbp_imp (* (* (- (.ImpactPoint (Collision|BreakHitResult _outhit)) (Transformation|GetWorldLocation (Variables|/Script/Engine.Character|GetCapsuleComponent (Game|GetPlayerCharacter 0)))) (Variables|Default|GetWind%20Strength)) 2.0) true true)
        (else
          (bind _asbp_ground_piece (Utilities|Casting|CastToBP_Ground_Piece (.HitActor (Collision|BreakHitResult _outhit))))
          (Default|DropGroundPiece _asbp_ground_piece)
          (Physics|AddImpulse (.HitComponent (Collision|BreakHitResult _outhit)) (* (- (.ImpactPoint (Collision|BreakHitResult _outhit)) (Transformation|GetWorldLocation (Variables|/Script/Engine.Character|GetCapsuleComponent (Game|GetPlayerCharacter 0)))) (Variables|Default|GetWind%20Strength)) "None" true))))))

(fn ConstructionScript
  (|CallParentFunction))