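; Water bubble magic projectile that flies forward, bursts on WorldStatic geometry and captures living Imps or ground pieces it overlaps.
; A catch snaps to a tumbling attach point, and shortly afterwards the bubble also drifts upward.
; After HoldLifetime it bursts, restoring Imp movement and collision or releasing the piece into physics.
; Timelines animate spawn, attach and burst scale with Niagara and sound effects, and WindPush offsets the bubble.
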(event OnComponentBeginOverlap(Bubble)
  (params (OverlappedComponent :type Primitive%20Component%20Object%20Reference) (OtherActor :type Actor%20Object%20Reference) (OtherComp :type Primitive%20Component%20Object%20Reference) (OtherBodyIndex :type Integer) (bFromSweep :type Boolean) (SweepResult :type Hit%20Result%20Structure%20%28by%20ref%29))
  ;[1 1 1] Grab Imp
  (if (Utilities|Enum|Equal(Enum) (Collision|GetCollisionObjectType OtherComp) "ECC_WorldStatic")
    (CallFunction|CollisionBurst)
    (else
      (Utilities|Casting|CastToBP_FirstPersonCharacter OtherActor
        (:CastFailed
          (if (Utilities|DoesObjectImplementInterface OtherActor "/Game/Blueprints/AI/BPI_Enemy.BPI_Enemy_C")
            (bind _asbp_imp (Utilities|Casting|CastToBP_Imp OtherActor))
            (if (not (Variables|/Game/Blueprints/AI/BP_Imp.BP_Imp_C|GetDead _asbp_imp))
              (Utilities|FlowControl|DoOnce false
                (:Completed
                  (Collision|SetCollisionEnabled (Variables|Default|GetBubble) "NoCollision")
                  (Collision|SetCollisionEnabled (Variables|/Script/Engine.Character|GetCapsuleComponent _asbp_imp) "NoCollision")
                  (Default|ToggleMovement _asbp_imp)
                  (Transformation|AttachComponentToComponent _asbp_imp (Variables|Default|GetImp%20Attach%20Point) "None" "SnapToTarget" "SnapToTarget" "SnapToTarget" true)
                  (Variables|/Game/Blueprints/AI/BP_Imp.BP_Imp_C|SetIn%20Bubble _asbp_imp true)
                  (CallFunction|Attach)
                  (CallFunction|ChangeMovement)
                  (Components|Activation|Activate (Variables|Default|GetNiagara) false)
                  (Audio|PlaySoundatLocation "/Game/Audio/SC_Bubble_Attach.SC_Bubble_Attach" (Transformation|GetActorLocation) "0, 0, 0" 1.0 1.0 0.0 0 0 0 0)
                  (CallFunction|StartRotating)
                  (CallFunction|DropEnemy))))
            (else
              ;[1 1 1] Grab Ground Piece
              (bind _asbp_ground_piece (Utilities|Casting|CastToBP_Ground_Piece OtherActor))
              (Utilities|FlowControl|DoOnce false
                (:Completed
                  (Default|DropGroundPiece _asbp_ground_piece)
                  (Transformation|AttachComponentToComponent (Variables|/Game/Blueprints/Magic/BP_Ground_Piece.BP_Ground_Piece_C|GetStaticMesh _asbp_ground_piece) (Variables|Default|GetImp%20Attach%20Point) "None" "SnapToTarget" "SnapToTarget" "KeepWorld" true)
                  (CallFunction|Attach)
                  (CallFunction|ChangeMovement)
                  (Components|Activation|Activate (Variables|Default|GetNiagara) false)
                  (Audio|PlaySoundatLocation "/Game/Audio/SC_Bubble_Attach.SC_Bubble_Attach" (Transformation|GetActorLocation) "0, 0, 0" 1.0 1.0 0.0 0 0 0 0)
                  (CallFunction|StartRotating)
                  (CallFunction|DropGroundPiece))))))))))

(event Custom|Collision%20Burst
  (bind _returnvalue (Transformation|GetActorLocation))
  ;[1 1 1] Collision
  (Utilities|FlowControl|DoOnce false
    (:Completed
      (Niagara|SpawnSystematLocation "/Game/VFX/NS_Water_Hit.NS_Water_Hit" (Transformation|GetActorLocation))
      (Components|Activation|Deactivate (Variables|Default|GetNiagara))
      (Audio|PlaySoundatLocation "/Game/Audio/SC_Bubble_Burst.SC_Bubble_Burst" _returnvalue "0, 0, 0" 1.0 1.0 0.0 0 0 0 0)
      (Audio|PlaySoundatLocation "/Game/Audio/SC_Bubble_Spawn.SC_Bubble_Spawn" _returnvalue "0, 0, 0" 1.0 1.0 0.0 0 0 0 0)
      (CallFunction|Burst)
      (Utilities|FlowControl|Delay 0.2)
      (Actor|DestroyActor))))

(event Custom|Start%20Rotating
  ;[1 1 1] Rotate Imp
  (Timeline|Timeline PlayFromStart
    (:Update
      (Transformation|AddLocalRotation (Variables|Default|GetImp%20Attach%20Point) "-0.200000,0.200000,0.200000" false false))))

(event Custom|Drop%20Enemy
  (bind _returnvalue (Transformation|GetActorLocation))
  ;[1 1 1] Drop Enemy
  (Utilities|FlowControl|Delay (Variables|Default|GetHold%20Lifetime))
  (Niagara|SpawnSystematLocation "/Game/VFX/NS_Water_Hit.NS_Water_Hit" (Transformation|GetActorLocation))
  (Transformation|DetachFromActor (stale OnComponentBeginOverlap(Bubble) _asbp_imp) "KeepWorld" "KeepWorld" "KeepWorld")
  (Collision|SetCollisionEnabled (Variables|Default|GetBubble) "NoCollision")
  (Collision|SetCollisionEnabled (Variables|/Script/Engine.Character|GetCapsuleComponent (stale OnComponentBeginOverlap(Bubble) _asbp_imp)) "QueryAndPhysics")
  (Default|ToggleMovement (stale OnComponentBeginOverlap(Bubble) _asbp_imp))
  (Variables|/Game/Blueprints/AI/BP_Imp.BP_Imp_C|SetIn%20Bubble (stale OnComponentBeginOverlap(Bubble) _asbp_imp) false)
  (Variables|/Game/Blueprints/AI/BP_Imp.BP_Imp_C|SetBubble%20Drop (stale OnComponentBeginOverlap(Bubble) _asbp_imp) true)
  (Components|Activation|Deactivate (Variables|Default|GetNiagara))
  (Audio|PlaySoundatLocation "/Game/Audio/SC_Bubble_Burst.SC_Bubble_Burst" _returnvalue "0, 0, 0" 1.0 1.0 0.0 0 0 0 0)
  (Audio|PlaySoundatLocation "/Game/Audio/SC_Bubble_Spawn.SC_Bubble_Spawn" _returnvalue "0, 0, 0" 1.0 1.0 0.0 0 0 0 0)
  (CallFunction|Burst)
  (Utilities|FlowControl|Delay 0.5)
  (Actor|DestroyActor))

(event Custom|Wind%20Push
  (params (Hit%20Direction :type Vector))
  (Variables|Default|SetWind%20Pushing true)
  (Transformation|AddActorWorldOffset (* Hit%20Direction (Variables|Default|GetWind%20Push%20Factor))))

(event Custom|Spawn
  ;[1 1 1] Animations
  (bind _scale (Timeline|Bubble_Spawn PlayFromStart)
    (:Update
      (Transformation|SetRelativeScale3D (Variables|Default|GetBubble) _scale))))

(event Custom|Burst
  ;[1 1 1] Animations
  (bind _scale (Timeline|Bubble_Burst PlayFromStart)
    (:Update
      (Transformation|SetRelativeScale3D (Variables|Default|GetBubble) _scale))))

(event Custom|Attach
  ;[1 1 1] Animations
  (bind _scale (Timeline|Bubble_Attach PlayFromStart)
    (:Update
      (Transformation|SetRelativeScale3D (Variables|Default|GetBubble) _scale))))

(event Custom|Change%20Movement
  ;[1 1 1] Change Movement
  (Utilities|FlowControl|Delay 0.5)
  (Variables|Default|SetAttached true))

(event Custom|Drop%20Ground%20Piece
  (bind _returnvalue (Transformation|GetActorLocation))
  ;[1 1 1] Drop Ground Piece
  (Utilities|FlowControl|Delay (Variables|Default|GetHold%20Lifetime))
  (Niagara|SpawnSystematLocation "/Game/VFX/NS_Water_Hit.NS_Water_Hit" (Transformation|GetActorLocation))
  (Collision|SetCollisionEnabled (Variables|Default|GetBubble) "NoCollision")
  (Transformation|DetachFromComponent (Variables|/Game/Blueprints/Magic/BP_Ground_Piece.BP_Ground_Piece_C|GetStaticMesh (stale OnComponentBeginOverlap(Bubble) _asbp_ground_piece)) "KeepWorld" "KeepWorld" "KeepWorld" false)
  (Default|DropGroundPiece (stale OnComponentBeginOverlap(Bubble) _asbp_ground_piece))
  (Collision|SetCollisionEnabled (Variables|/Game/Blueprints/Magic/BP_Ground_Piece.BP_Ground_Piece_C|GetStaticMesh (stale OnComponentBeginOverlap(Bubble) _asbp_ground_piece)) "QueryAndPhysics")
  (Physics|SetSimulatePhysics (Variables|/Game/Blueprints/Magic/BP_Ground_Piece.BP_Ground_Piece_C|GetStaticMesh (stale OnComponentBeginOverlap(Bubble) _asbp_ground_piece)) true)
  (Collision|SetCollisionProfileName (Variables|/Game/Blueprints/Magic/BP_Ground_Piece.BP_Ground_Piece_C|GetStaticMesh (stale OnComponentBeginOverlap(Bubble) _asbp_ground_piece)) "PhysicsActor" true :!class /Script/Engine.PrimitiveComponent)
  (Physics|SetEnableGravity (Variables|/Game/Blueprints/Magic/BP_Ground_Piece.BP_Ground_Piece_C|GetStaticMesh (stale OnComponentBeginOverlap(Bubble) _asbp_ground_piece)) true)
  (Class|PrimitiveComponent|SetNotifyRigidBodyCollision (Variables|/Game/Blueprints/Magic/BP_Ground_Piece.BP_Ground_Piece_C|GetStaticMesh (stale OnComponentBeginOverlap(Bubble) _asbp_ground_piece)) true)
  (Rendering|SetRenderCustomDepth (Variables|/Game/Blueprints/Magic/BP_Ground_Piece.BP_Ground_Piece_C|GetStaticMesh (stale OnComponentBeginOverlap(Bubble) _asbp_ground_piece)) false)
  (Components|Activation|Deactivate (Variables|Default|GetNiagara))
  (Audio|PlaySoundatLocation "/Game/Audio/SC_Bubble_Burst.SC_Bubble_Burst" _returnvalue "0, 0, 0" 1.0 1.0 0.0 0 0 0 0)
  (Audio|PlaySoundatLocation "/Game/Audio/SC_Bubble_Spawn.SC_Bubble_Spawn" _returnvalue "0, 0, 0" 1.0 1.0 0.0 0 0 0 0)
  (CallFunction|Burst)
  (Utilities|FlowControl|Delay 0.2)
  (Actor|DestroyActor))

(event EventTick
  (params (DeltaSeconds :type Float%20%28single-precision%29))
  (bind _returnvalue (Transformation|GetActorForwardVector))
  ;[1 1 1] Movement
  (if (Variables|Default|GetAttached)
    (Transformation|AddActorWorldOffset (* (+ (Math|Vector|VectorUp) _returnvalue) (Variables|Default|GetMove%20Speed)))
    (else
      (Transformation|AddActorWorldOffset (* _returnvalue (Variables|Default|GetMove%20Speed))))))

(event EventBeginPlay
  (CallFunction|Spawn))

(fn ConstructionScript)