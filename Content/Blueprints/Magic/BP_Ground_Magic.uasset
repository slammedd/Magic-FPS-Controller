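; Ground magic spell that pulls a rock piece out of the landscape, then drops it on the next cast.
; Casting traces from the player camera; a Landscape hit plays sound and VFX and spawns a randomly rotated BP_Ground_Piece.
; Casting while RockHeld drops the piece, clears the flag and resets the character's GroundPieceContainer to its forward offset.
; RockHeld is only cleared here, never set.
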(event EventStartCasting
  (bind _returnvalue (Game|GetPlayerCameraManager 0))
  (bind _transformcomponent (Variables|/Script/Engine.PlayerCameraManager|GetTransformComponent _returnvalue))
  (bind _returnvalue_2 (Math|Vector|GetForwardVector _transformcomponent))
  (bind _returnvalue_3 (Transformation|GetWorldLocation _transformcomponent))
  (bind _returnvalue_4 (+ _returnvalue_3 _returnvalue_2))
  (if (Variables|Default|GetRock%20Held)
    (Audio|PlaySoundatLocation "/Game/Audio/SC_Ground_Magic_End.SC_Ground_Magic_End" (Transformation|GetWorldLocation (Variables|/Script/Engine.Character|GetCapsuleComponent (Game|GetPlayerCharacter 0))) "0, 0, 0" 1.0 1.0 0.0 0 0 0 0)
    (Default|DropGroundPiece (Variables|Default|GetGround%20Piece))
    (Variables|Default|SetRock%20Held false)
    (bind _asbp_first_person_character (Utilities|Casting|CastToBP_FirstPersonCharacter (Game|GetPlayerCharacter 0)))
    (Transformation|SetRelativeLocation (Variables|/Game/Blueprints/BP_FirstPersonCharacter.BP_FirstPersonCharacter_C|GetGround%20Piece%20Container _asbp_first_person_character) "1000.000000,0.000000,0.000000" false true)
    (else
      (bind (_outhit _returnvalue_5) (Collision|LineTraceByChannel _returnvalue_4 (+ _returnvalue_4 (* _returnvalue_2 (Variables|Default|GetCast%20Distance))) "TraceTypeQuery1" false 0 "None"))
      (if _returnvalue_5
        (switch Utilities|FlowControl|Switch|SwitchonECollisionChannel (Collision|GetCollisionObjectType (.HitComponent (Collision|BreakHitResult _outhit)))
          (:ECC_GameTraceChannel2
            (Audio|PlaySoundatLocation "/Game/Audio/SC_Ground_Magic_Hit.SC_Ground_Magic_Hit" (Transformation|GetWorldLocation (Variables|/Script/Engine.Character|GetCapsuleComponent (Game|GetPlayerCharacter 0))) "0, 0, 0" 1.0 1.0 0.0 0 0 0 0)
            (Components|Activation|Activate (Variables|Default|GetMagic%20VFX) false)
            (bind _returnvalue_6 (Game|SpawnActorfromClass "/Game/Blueprints/Magic/BP_Ground_Piece.BP_Ground_Piece_C" (Math|Transform|MakeTransform (.Location (Collision|BreakHitResult _outhit)) "0, 0, 0" "1.000000,1.000000,1.000000") "AlwaysSpawn" "MultiplyWithRoot" 0 0))
            (bind _output_get (Variables|Default|SetGround%20Piece _returnvalue_6))
            (Transformation|SetRelativeRotation (Variables|/Game/Blueprints/Magic/BP_Ground_Piece.BP_Ground_Piece_C|GetStaticMesh _output_get) (Math|Random|RandomRotator true) false false)))))))

(fn ConstructionScript
  (|CallParentFunction))