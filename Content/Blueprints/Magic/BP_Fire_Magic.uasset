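; Fire magic spell that streams a VFX flame while casting and forward-traces every tick to find what it hits.
; Actors implementing BPI_Enemy receive a hit message each tick, with a coin-flip chance of being set on fire.
; Water bubbles drop their attached enemy or ground piece, or burst if nothing is attached.
; Wind-affected and normal speed events switch the particle rate, velocity, cone and cast distance.
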(event Custom|Normal%20Speed
  (bind _magic_vfx (Variables|Default|GetMagic%20VFX))
  (Niagara|SetNiagaraVariable(Float) _magic_vfx "Spawn Rate" 4e+01)
  (Niagara|SetNiagaraVariable(Float) _magic_vfx "Min Velocity" 1.5e+03)
  (Niagara|SetNiagaraVariable(Float) _magic_vfx "Max Velocity" 2.5e+03)
  (Niagara|SetNiagaraVariable(Float) _magic_vfx "Cone Angle" 5.0)
  (Variables|Default|SetCast%20Distance 1.5e+03))

(event Custom|Wind%20Affected%20Speed
  (bind _magic_vfx (Variables|Default|GetMagic%20VFX))
  (Niagara|SetNiagaraVariable(Float) _magic_vfx "Spawn Rate" 8e+01)
  (Niagara|SetNiagaraVariable(Float) _magic_vfx "Min Velocity" 2.5e+03)
  (Niagara|SetNiagaraVariable(Float) _magic_vfx "Max Velocity" 4.5e+03)
  (Niagara|SetNiagaraVariable(Float) _magic_vfx "Cone Angle" 1e+01)
  (Variables|Default|SetCast%20Distance 2.5e+03))

(event EventStartCasting
  (Components|Activation|Activate (Variables|Default|GetMagic%20VFX) false)
  (Variables|Default|SetCasting true))

(event EventStopCasting
  (Components|Activation|Deactivate (Variables|Default|GetMagic%20VFX))
  (Variables|Default|SetCasting false))

(event EventTick
  (params (DeltaSeconds :type Float%20%28single-precision%29))
  (if (Variables|Default|GetCasting)
    (bind _hit_result (CallFunction|TraceForward))
    (if (Utilities|DoesObjectImplementInterface (.HitActor (Collision|BreakHitResult _hit_result)) "/Game/Blueprints/AI/BPI_Enemy.BPI_Enemy_C")
      ;[1 1 1] Hit Enemy
      (Class|BPIEnemy|EnemyHit(Message) (.HitActor (Collision|BreakHitResult _hit_result)) 25.0)
      (if (== (Math|Random|RandomIntegerinRange 0 1) 0)
        (Class|BPIEnemy|StartFire(Message) (.HitActor (Collision|BreakHitResult _hit_result))))
      (else
        ;[1 1 1] Hit Bubble
        (bind _asbp_water_bubble (Utilities|Casting|CastToBP_Water_Bubble (.HitActor (Collision|BreakHitResult _hit_result))))
        (if (Variables|/Game/Blueprints/Magic/BP_Water_Bubble.BP_Water_Bubble_C|GetAttached _asbp_water_bubble)
          (Default|DropEnemy _asbp_water_bubble)
          (Default|DropGroundPiece _asbp_water_bubble)
          (else
            (Default|CollisionBurst _asbp_water_bubble)))))))

(fn ConstructionScript
  (|CallParentFunction))