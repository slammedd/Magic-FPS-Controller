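; Rock piece for the player's ground magic that can be held, dropped and smashed to damage enemies.
; On spawn it rises with smoke, interpolates to the player's GroundPieceContainer, then attaches through GrabConstraint.
; Dropping breaks the constraint and restores gravity and hit notifications.
; A hit above the impulse threshold plays a scale timeline, then hides the rock and sphere-traces to send damage through BPI_Enemy.
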(event OnComponentHit(StaticMesh)
  (params (HitComponent :type Primitive%20Component%20Object%20Reference) (OtherActor :type Actor%20Object%20Reference) (OtherComp :type Primitive%20Component%20Object%20Reference) (NormalImpulse :type Vector :default "0, 0, 0") (Hit :type Hit%20Result%20Structure%20%28by%20ref%29))
  (bind _location (Collision|BreakHitResult Hit))
  (bind _staticmesh (Variables|Default|GetStaticMesh))
  ;[1 1 1] Break Rock
  (if (not (Variables|Default|GetBroken))
    (if (>= (Math|Vector|VectorLength NormalImpulse) (Variables|Default|GetBreak%20Threshold%20Velocity))
      (Variables|Default|SetBroken true)
      (Audio|PlaySoundatLocation "/Game/Audio/SC_Rock_Smash.SC_Rock_Smash" _location "0, 0, 0" 1.0 1.0 0.0 0 0 0 0)
      (bind _scale (Timeline|Scale PlayFromStart)
        (:Update
          (Transformation|SetRelativeScale3D (Variables|Default|GetStaticMesh) _scale))
        (:Finished
          (Audio|PlaySoundatLocation "/Game/Audio/SC_Ground_Magic_Hit.SC_Ground_Magic_Hit" _location "0, 0, 0" 1.0 1.0 0.0 0 0 0 0)
          (Niagara|SpawnSystematLocation "/Game/VFX/NS_Ground_Magic_Hit.NS_Ground_Magic_Hit" _location "0, 0, 0" "3.000000,3.000000,3.000000")
          (Development|SetHiddeninGame (Variables|Default|GetStaticMesh) true false)
          (bind (_outhits _returnvalue) (Collision|MultiSphereTraceByChannel _location _location (Variables|Default|GetDamage%20Radius) "TraceTypeQuery1" false 0 "None"))
          (if _returnvalue
            (bind _array_element (Utilities|Array|ForEachLoopwithBreak _outhits)
              (:LoopBody
                (if (Utilities|DoesObjectImplementInterface (.HitActor (Collision|BreakHitResult _array_element)) "/Game/Blueprints/AI/BPI_Enemy.BPI_Enemy_C")
                  (Class|BPIEnemy|EnemyHit(Message) (.HitActor (Collision|BreakHitResult _array_element)) (Variables|Default|GetDamage))
                  (Physics|SetSimulatePhysics _staticmesh false)
                  (Collision|SetCollisionEnabled _staticmesh "NoCollision"))))))))))

(event OnComponentBeginOverlap(CollsionSound)
  (params (OverlappedComponent :type Primitive%20Component%20Object%20Reference) (OtherActor :type Actor%20Object%20Reference) (OtherComp :type Primitive%20Component%20Object%20Reference) (OtherBodyIndex :type Integer) (bFromSweep :type Boolean) (SweepResult :type Hit%20Result%20Structure%20%28by%20ref%29))
  ;[1 1 1] Hit Sound
  (if (not (and (Variables|Default|GetInterpolating) (!= OtherComp (Variables|Default|GetStaticMesh))))
    (if (Variables|Default|GetCan%20Play%20Hit%20Sound)
      (Utilities|Casting|CastToBP_FirstPersonCharacter OtherActor
        (:CastFailed
          ;[1 1 1] Check if enemy
          (if (Utilities|DoesObjectImplementInterface (.HitActor (Collision|BreakHitResult SweepResult)) "/Game/Blueprints/AI/BPI_Enemy.BPI_Enemy_C")
            (Class|PrimitiveComponent|SetNotifyRigidBodyCollision (Variables|Default|GetStaticMesh) true)))))))

(event Custom|Spawn%20Animation
  (bind _staticmesh (Variables|Default|GetStaticMesh))
  ;[1 1 1] Rock Spawn Animation
  (bind _z (Timeline|Location PlayFromStart)
    (:Update
      (Transformation|AddActorWorldOffset _z))
    (:Finished
      (Collision|SetCollisionEnabled _staticmesh "PhysicsOnly")
      (Physics|SetSimulatePhysics _staticmesh true)
      (Collision|SetCollisionProfileName _staticmesh "PhysicsActor" true :!class /Script/Engine.PrimitiveComponent)
      (Physics|SetEnableGravity _staticmesh false)
      (Components|Activation|Deactivate (stale EventBeginPlay _returnvalue))
      (Variables|Default|SetInterpolating true)
      (Rendering|SetRenderCustomDepth (Variables|Default|GetStaticMesh) true))))

(event Custom|Drop%20Ground%20Piece
  (bind _staticmesh (Variables|Default|GetStaticMesh))
  ;[1 1 1] Drop Ground Piece
  (Variables|Default|SetCan%20Play%20Hit%20Sound false)
  (bind _asbp_first_person_character (Utilities|Casting|CastToBP_FirstPersonCharacter (Game|GetPlayerCharacter 0)))
  (bind _asbp_ground_magic (Utilities|Casting|CastToBP_Ground_Magic (Variables|/Game/Blueprints/BP_FirstPersonCharacter.BP_FirstPersonCharacter_C|GetCurrent%20Left%20Hand%20Magic _asbp_first_person_character))
    (:then
      (Components|Activation|Deactivate (Variables|/Game/Blueprints/Magic/BP_Base_Magic.BP_Base_Magic_C|GetMagic%20VFX _asbp_ground_magic)))
    (:CastFailed
      (bind _asbp_ground_magic_2 (Utilities|Casting|CastToBP_Ground_Magic (Variables|/Game/Blueprints/BP_FirstPersonCharacter.BP_FirstPersonCharacter_C|GetCurrent%20Right%20Hand%20Magic _asbp_first_person_character)))
      (Components|Activation|Deactivate (Variables|/Game/Blueprints/Magic/BP_Base_Magic.BP_Base_Magic_C|GetMagic%20VFX _asbp_ground_magic_2))))
  (Class|PhysicsConstraintComponent|BreakConstraint (Variables|/Game/Blueprints/BP_FirstPersonCharacter.BP_FirstPersonCharacter_C|GetGrab%20Constraint (Variables|Default|GetPlayer)))
  (Collision|SetCollisionEnabled _staticmesh "QueryAndPhysics")
  (Collision|SetCollisionProfileName _staticmesh "PhysicsActor" true :!class /Script/Engine.PrimitiveComponent)
  (Physics|SetEnableGravity _staticmesh true)
  (Class|PrimitiveComponent|SetNotifyRigidBodyCollision _staticmesh true)
  (Rendering|SetRenderCustomDepth _staticmesh false))

(event EventBeginPlay
  (bind _asbp_first_person_character (Utilities|Casting|CastToBP_FirstPersonCharacter (Game|GetPlayerCharacter 0)))
  (Variables|Default|SetPlayer _asbp_first_person_character)
  (bind _outactors (Actor|GetAllActorsOfClass "/Game/Blueprints/Magic/BP_Ground_Magic.BP_Ground_Magic_C"))
  (Variables|Default|SetGround%20Magic (Utilities|Array|Get(acopy) _outactors))
  (Audio|PlaySoundatLocation "/Game/Audio/SC_Rock_Spawn.SC_Rock_Spawn" (Transformation|GetWorldLocation (Variables|Default|GetDefaultSceneRoot)) "0, 0, 0" 1.0 1.0 0.0 0 0 0 0)
  (CallFunction|SpawnAnimation)
  (bind _returnvalue (Niagara|SpawnSystematLocation "/Game/VFX/NS_Ground_Smoke.NS_Ground_Smoke" (Transformation|GetWorldLocation (Variables|Default|GetDefaultSceneRoot)))))

(event EventTick
  (params (DeltaSeconds :type Float%20%28single-precision%29))
  (bind _staticmesh (Variables|Default|GetStaticMesh))
  (bind _player (Variables|Default|GetPlayer))
  (if (Variables|Default|GetInterpolating)
    (Transformation|SetWorldLocation _staticmesh (Math|Interpolation|VInterpTo (Transformation|GetWorldLocation _staticmesh) (Transformation|GetWorldLocation (Variables|/Game/Blueprints/BP_FirstPersonCharacter.BP_FirstPersonCharacter_C|GetGround%20Piece%20Container (Variables|Default|GetPlayer))) (Utilities|Time|GetWorldDeltaSeconds) (Variables|Default|GetHold%20Interp%20Speed)) false true)
    (Utilities|FlowControl|Delay 0.5)
    (Variables|Default|SetInterpolating false)
    (Class|PhysicsConstraintComponent|SetConstrainedComponents (Variables|/Game/Blueprints/BP_FirstPersonCharacter.BP_FirstPersonCharacter_C|GetGrab%20Constraint _player) (Variables|Default|GetStaticMesh) "None" (Variables|/Game/Blueprints/BP_FirstPersonCharacter.BP_FirstPersonCharacter_C|GetGround%20Piece%20Container _player) "None")
    (Class|PrimitiveComponent|SetNotifyRigidBodyCollision (Variables|Default|GetStaticMesh) false)
    (Variables|/Game/Blueprints/Magic/BP_Ground_Magic.BP_Ground_Magic_C|SetRock%20Held (Variables|Default|GetGround%20Magic) true)
    (Variables|Default|SetCan%20Play%20Hit%20Sound true)))

(fn ConstructionScript)