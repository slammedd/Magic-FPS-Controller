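; A pressure button that spawns a single enemy when the first-person player character steps on it.
; Overlap plays a click sound and a timeline that moves and scales the button mesh.
; It then calls Spawn1 on the first BP_Enemy_Spawner found in the level.
; An IsSpawning flag blocks repeat presses until ResetSpawning clears it.
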(event OnComponentBeginOverlap(StaticMesh1)
  (params (OverlappedComponent :type Primitive%20Component%20Object%20Reference) (OtherActor :type Actor%20Object%20Reference) (OtherComp :type Primitive%20Component%20Object%20Reference) (OtherBodyIndex :type Integer) (bFromSweep :type Boolean) (SweepResult :type Hit%20Result%20Structure%20%28by%20ref%29))
  (if (not (Variables|Default|GetIs%20Spawning))
    (Utilities|Casting|CastToBP_FirstPersonCharacter OtherActor)
    (Variables|Default|SetIs%20Spawning true)
    (CallFunction|ButtonPressed)
    (bind _outactors (Actor|GetAllActorsOfClass "/Game/Blueprints/AI/BP_Enemy_Spawner.BP_Enemy_Spawner_C"))
    (Default|Spawn1 (Utilities|Array|Get(acopy) _outactors))))

(event Custom|Reset%20Spawning
  (Variables|Default|SetIs%20Spawning false))

(event Custom|Button%20Pressed
  (Audio|PlaySoundatLocation "/Game/Audio/SC_Button_Click.SC_Button_Click" (Transformation|GetActorLocation) "0, 0, 0" 1.0 1.0 0.0 0 0 0 0)
  (bind (_direction _location _scale) (Timeline|Pressed%20Animation PlayFromStart)
    (:Update
      (Transformation|SetRelativeTransform (Variables|Default|GetStaticMesh1) (Math|Transform|MakeTransform _location "0, 0, 0" _scale) false false))))

(fn ConstructionScript)