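; BP_Demon is an AI enemy character that shoots projectiles at the player and can be set on fire.
; It toggles a "Can Move" Blackboard key on spawn, death and player detection, where overlap starts a looping attack-montage timer and AttackTrace spawns the projectile.
; Hits, timed burn ticks and BubbleDrop landings drain health, ending in ragdoll, smoke and shrink-out.
; Tick traces the ground to pick grass or dirt footstep sounds.
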(event OnComponentBeginOverlap(PlayerDetection)
  (params (OverlappedComponent :type Primitive%20Component%20Object%20Reference) (OtherActor :type Actor%20Object%20Reference) (OtherComp :type Primitive%20Component%20Object%20Reference) (OtherBodyIndex :type Integer) (bFromSweep :type Boolean) (SweepResult :type Hit%20Result%20Structure%20%28by%20ref%29))
  ;[1 1 1] Attack
  (Utilities|Casting|CastToBP_FirstPersonCharacter OtherActor)
  (Utilities|FlowControl|DoOnce false
    (:Completed
      (Utilities|FlowControl|Delay 0.2)
      (AI|Components|Blackboard|SetValueasBool (AI|GetBlackboard 0) (Utilities|Name|MakeLiteralName "Can Move") false)
      (bind _returnvalue (Utilities|Time|SetTimerbyEvent (delegate Custom|Attack%20Player) (Variables|Default|GetAttack%20Cooldown) true)))))

(event OnComponentEndOverlap(PlayerDetection)
  (params (OverlappedComponent :type Primitive%20Component%20Object%20Reference) (OtherActor :type Actor%20Object%20Reference) (OtherComp :type Primitive%20Component%20Object%20Reference) (OtherBodyIndex :type Integer))
  (bind _returnvalue (AI|GetBlackboard 0))
  (bind _returnvalue_2 (Utilities|Name|MakeLiteralName "Can Move"))
  ;[1 1 1] Attack
  (Utilities|Casting|CastToBP_FirstPersonCharacter OtherActor)
  (Utilities|Time|ClearandInvalidateTimerbyHandle (stale OnComponentBeginOverlap(PlayerDetection) _returnvalue))
  (AI|Components|Blackboard|SetValueasBool _returnvalue _returnvalue_2 true)
  (Utilities|FlowControl|DoOnce false) ; enters at Reset
)

(event Custom|Footstep%20Sound
  ;[1 1 1] Footstep Sounds
  (CallFunction|CheckPhyscialMaterial)
  (if (and (!= (Math|Vector|VectorLength (Transformation|GetVelocity)) 0.0) (not (AI|Components|NavMovement|IsFalling (Variables|Character|GetCharacterMovement))))
    (Utilities|FlowControl|DoOnce false :!label _label
      (:Completed
        (bind _returnvalue (Utilities|Time|SetTimerbyEvent (delegate Custom|Play%20Footstep%20Sound) (Variables|Default|GetFootstep%20Interval) true))))
    (else
      (Utilities|Time|ClearandInvalidateTimerbyHandle _returnvalue)
      (goto _label Reset))))

(event Custom|Attack%20Player
  ;[1 1 1] Attack
  (Animation|PlayAnimMontage "/Game/Animations/AM_Attack.AM_Attack" 1.0 "None"))

(event Custom|Attack%20Trace
  (bind _mesh (Variables|Character|GetMesh))
  (bind _returnvalue (Transformation|GetWorldLocation _mesh))
  (bind _returnvalue_2 (+ (.z _returnvalue) 125.0))
  (bind _returnvalue_3 (Math|Vector|MakeVector (.x _returnvalue) (.y _returnvalue) _returnvalue_2))
  ;[1 1 1] Attack
  (Game|SpawnActorfromClass "/Game/Blueprints/AI/BP_Demon_Projectile.BP_Demon_Projectile_C" (Math|Transform|MakeTransform (+ _returnvalue_3 (* (Math|Vector|GetForwardVector _mesh) 1.2)) (Math|Rotator|FindLookatRotation _returnvalue_3 (Transformation|GetActorLocation (Game|GetPlayerCharacter 0))) "1.000000,1.000000,1.000000") "Undefined" "MultiplyWithRoot" 0 0))

(event Custom|Look%20at%20Player
  ;[1 1 1] Look at Player
  (Transformation|SetWorldRotation (Variables|Collision|GetCapsuleComponent) (Math|Rotator|FindLookatRotation (Transformation|GetWorldLocation (Variables|Collision|GetCapsuleComponent)) (Transformation|GetWorldLocation (Variables|/Script/Engine.Character|GetCapsuleComponent (Game|GetPlayerCharacter 0)))) false false))

(event Custom|Play%20Footstep%20Sound
  ;[1 1 1] Footstep Sounds
  (Audio|PlaySoundatLocation (Variables|Default|GetFootstep%20SFX) (- (Transformation|GetActorLocation) "0.000000,0.000000,44.000000") "0, 0, 0" 0.3 1.2 0.0 0 0 0 0))

(event Custom|Check%20Physcial%20Material
  (bind _returnvalue (Transformation|GetActorLocation))
  ;[1 1 1] Footstep Sounds
  (bind (_outhit _returnvalue_2) (Collision|LineTraceByChannel _returnvalue (- _returnvalue "0.000000,0.000000,144.000000") "TraceTypeQuery1" false 0 "None"))
  (if _returnvalue_2
    (switch Utilities|FlowControl|Switch|SwitchonEPhysicalSurface (Collision|GetSurfaceType _outhit)
      (:SurfaceType1
        (Variables|Default|SetFootstep%20SFX "/Game/Audio/SC_Grass_Footstep.SC_Grass_Footstep"))
      (:SurfaceType2
        (Variables|Default|SetFootstep%20SFX "/Game/Audio/SC_Dirt_Footsteps.SC_Dirt_Footsteps")))))

(event Custom|Spawn
  (bind _returnvalue (Transformation|GetActorLocation))
  ;[1 1 1] Spawn
  (Audio|PlaySoundatLocation "/Game/Audio/SC_Imp_Spawn.SC_Imp_Spawn" _returnvalue "0, 0, 0" 1.0 1.0 0.0 0 0 0 0)
  (Audio|PlaySoundatLocation "/Game/Audio/SC_Smoke_Poof.SC_Smoke_Poof" _returnvalue "0, 0, 0" 1.0 1.0 0.0 0 0 0 0)
  (Utilities|FlowControl|Delay 2.1)
  (CallFunction|ToggleMovement)
  (Components|Activation|Deactivate (Variables|Default|GetSpawn%20Smoke)))

(event Custom|Die
  (bind _mesh (Variables|Character|GetMesh))
  (bind _mesh_2 (Variables|Character|GetMesh))
  (bind _returnvalue (Transformation|GetWorldLocation _mesh_2))
  ;[1 1 1] Die
  (AI|Components|Blackboard|SetValueasBool (Variables|Default|GetBlackboard) (Utilities|Name|MakeLiteralName "Can Move") false)
  (Class|NavMovementComponent|StopActiveMovement (Variables|Character|GetCharacterMovement))
  (Variables|Default|SetDead true)
  (Audio|PlaySoundatLocation "/Game/Audio/SC_Imp_Die.SC_Imp_Die" (Transformation|GetWorldLocation (Variables|Character|GetMesh)) "0, 0, 0" 1.0 1.0 0.0 0 0 0 0)
  (Collision|SetCollisionProfileName _mesh "Ragdoll" true :!class /Script/Engine.PrimitiveComponent)
  (Physics|SetSimulatePhysics _mesh true)
  (Physics|AddImpulse _mesh "0.000000,0.000000,1250.000000" "None" true)
  (Collision|SetCollisionEnabled (Variables|Default|GetPlayer%20Detection) "NoCollision")
  (Collision|SetCollisionEnabled (Variables|Collision|GetCapsuleComponent) "NoCollision")
  (Utilities|FlowControl|Delay 2.0)
  (Niagara|SpawnSystematLocation "/Game/VFX/NS_Spawn_Smoke.NS_Spawn_Smoke" _returnvalue)
  (Audio|PlaySoundatLocation "/Game/Audio/SC_Smoke_Poof.SC_Smoke_Poof" _returnvalue "0, 0, 0" 1.0 1.0 0.0 0 0 0 0)
  (bind _scale (Timeline|Scale Play)
    (:Update
      (Transformation|SetRelativeScale3D (Variables|Character|GetMesh) _scale))
    (:Finished
      (Actor|DestroyActor))))

(event Custom|Toggle%20Movement
  (bind _returnvalue (Utilities|Name|MakeLiteralName "Can Move"))
  (bind _blackboard (Variables|Default|GetBlackboard))
  ;[1 1 1] Toggle Movement
  (if (ScalableFloat|GetValueasBool (Variables|Default|GetBlackboard) (Utilities|Name|MakeLiteralName "Can Move"))
    (Components|Movement|StopMovementImmediately (Variables|Character|GetCharacterMovement))
    (AI|Components|Blackboard|SetValueasBool _blackboard _returnvalue false)
    (else
      (AI|Components|Blackboard|SetValueasBool _blackboard _returnvalue true))))

(event Custom|Fire%20Timer
  ;[1 1 1] Fire
  (CallFunction|EnemyHit 25.0))

(event Custom|Stop%20Fire
  ;[1 1 1] Fire
  (Components|Activation|Deactivate (Variables|Default|GetFire))
  (Utilities|Time|ClearandInvalidateTimerbyHandle (stale EventStartFire _returnvalue))
  (Variables|Default|SetOn%20Fire false)
  (Audio|Components|Audio|FadeOut (stale EventStartFire _returnvalue_2) 1.0 0.0 "Linear" :!class /Script/Engine.AudioComponent))

(event EventBeginPlay
  (Variables|Default|SetBlackboard (AI|GetBlackboard (Pawn|GetController)))
  (CallFunction|Spawn)
  (CallFunction|LookatPlayer))

(event EventEnemyHit
  (params (Damage :type Float%20%28double-precision%29))
  ;[1 1 1] Enemy Hit
  (if (<= (Variables|Default|GetHealth) 0.0)
    (Utilities|FlowControl|DoOnce false
      (:Completed
        (CallFunction|Die)))
    (else
      (Utilities|FlowControl|DoOnce false :!label _label
        (:Completed
          (Variables|Default|SetHealth (- (Variables|Default|GetHealth) Damage))
          (Animation|PlayAnimMontage "/Game/Animations/AM_Imp_Hit.AM_Imp_Hit" 1.0 "None")
          (if (<= (Variables|Default|GetHealth) 0.0)
            (Utilities|FlowControl|DoOnce false
              (:Completed
                (CallFunction|Die)))
            (else
              (Utilities|FlowControl|Delay 0.4)
              (goto _label Reset))))))))

(event EventTick
  (params (DeltaSeconds :type Float%20%28single-precision%29))
  (CallFunction|FootstepSound))

(event EventStartFire
  ;[1 1 1] Fire
  (if (not (Variables|Default|GetOn%20Fire))
    (Variables|Default|SetOn%20Fire true)
    (Components|Activation|Activate (Variables|Default|GetFire) false)
    (bind _returnvalue (Utilities|Time|SetTimerbyEvent (delegate Custom|Fire%20Timer) (Variables|Default|GetFire%20Damage%20Cooldown) true))
    (bind _returnvalue_2 (Audio|SpawnSoundAttached "/Game/Audio/SC_Fire.SC_Fire" (Variables|Collision|GetCapsuleComponent) "None" "0, 0, 0" "0, 0, 0" "KeepRelativeOffset" false 1.0 1.0 0.0 0 0))
    (Audio|Components|Audio|FadeIn _returnvalue_2 1.0 0.15 0.0 "Linear" :!class /Script/Engine.AudioComponent)
    (Utilities|FlowControl|RetriggerableDelay (Variables|Default|GetFire%20Duration))
    (CallFunction|StopFire)))

(event EventOnMovementModeChanged
  (params (PrevMovementMode :type EMovementMode%20Enum :default "MOVE_None") (NewMovementMode :type EMovementMode%20Enum :default "MOVE_None") (PrevCustomMode :type Byte :default 0) (NewCustomMode :type Byte :default 0))
  (if (Variables|Default|GetBubble%20Drop)
    (if (and (Utilities|Enum|Equal(Enum) PrevMovementMode "MOVE_Falling") (Utilities|Enum|Equal(Enum) NewMovementMode "MOVE_Walking"))
      (CallFunction|EnemyHit 1e+02))))

(fn ConstructionScript)