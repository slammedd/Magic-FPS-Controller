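; Enemy spawner actor that spawns either a single actor or a group of 25 imps, paired with spawner button actors.
; Spawn1 spawns at the BoxVisualisation component's location, while Spawn25 runs a fast looping timer that scatters BP_Imps randomly within a box around the root.
; When either spawn finishes, it calls ResetSpawning on the first matching single or group button found in the level.
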(event Custom|Spawn%2025
  (bind _returnvalue (Utilities|Time|SetTimerbyEvent (delegate Custom|Spawn%20Imp) 0.05 true)))

(event Custom|Spawn%201
  (Game|SpawnActorfromClass "/Game/Blueprints/AI/BP_Imp.BP_Imp_C" (Math|Transform|MakeTransform (Transformation|GetWorldLocation (Variables|Default|GetBox%20Visualisation)) "0, 0, 0" "1.000000,1.000000,1.000000") "AdjustIfPossibleButAlwaysSpawn" "MultiplyWithRoot" 0 0)
  (bind _outactors (Actor|GetAllActorsOfClass "/Game/Blueprints/AI/BP_Spawner_Button_Single_Enemy.BP_Spawner_Button_Single_Enemy_C"))
  (Default|ResetSpawning (Utilities|Array|Get(acopy) _outactors)))

(event Custom|Spawn%20Imp
  (if (>= (Variables|Default|GetSpawn%20Int) 25)
    (Utilities|Time|ClearandInvalidateTimerbyHandle (stale Custom|Spawn%2025 _returnvalue))
    (Variables|Default|SetSpawn%20Int 0)
    (bind _outactors (Actor|GetAllActorsOfClass "/Game/Blueprints/AI/BP_Spawner_Button_Group_Enemies.BP_Spawner_Button_Group_Enemies_C"))
    (Default|ResetSpawning (Utilities|Array|Get(acopy) _outactors))
    (else
      (Game|SpawnActorfromClass "/Game/Blueprints/AI/BP_Imp.BP_Imp_C" (Math|Transform|MakeTransform (Math|Random|RandomPointinBoundingBox (Transformation|GetWorldLocation (Variables|Default|GetDefaultSceneRoot)) "650.000000,650.000000,15.000000") "0, 0, 0" "1.000000,1.000000,1.000000") "AdjustIfPossibleButAlwaysSpawn" "MultiplyWithRoot" 0 0)
      (Math|Integer|IncrementInt (Variables|Default|GetSpawn%20Int)))))

(fn ConstructionScript)