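; Homing demon projectile that chases the player and bursts on contact.
; A timeline scales its Sphere from BeginPlay, while Tick re-sets the ProjectileMovement homing target to the player's capsule.
; Sphere hit and overlap share identical logic: spawn impact Niagara effect, play a sound and destroy the actor.
; Striking the player uses a different sound and adds camera shake, but the graph applies no damage.
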(event OnComponentHit(Sphere)
  (params (HitComponent :type Primitive%20Component%20Object%20Reference) (OtherActor :type Actor%20Object%20Reference) (OtherComp :type Primitive%20Component%20Object%20Reference) (NormalImpulse :type Vector :default "0, 0, 0") (Hit :type Hit%20Result%20Structure%20%28by%20ref%29))
  (bind _impactpoint (Collision|BreakHitResult Hit))
  (Utilities|Casting|CastToBP_FirstPersonCharacter OtherActor
    (:then
      (Audio|PlaySoundatLocation "/Game/Audio/SC_Bat_Hit.SC_Bat_Hit" _impactpoint "0, 0, 0" 1.0 1.0 0.0 0 0 0 0)
      (Niagara|SpawnSystematLocation "/Game/VFX/NS_Demon_Impact.NS_Demon_Impact" _impactpoint)
      (Class|LegacyCameraShake|StartLegacyCameraShake (Game|GetPlayerCameraManager 0) "/Game/Blueprints/BP_Take_Damage_Screen_Shake.BP_Take_Damage_Screen_Shake_C" 1.0 "CameraLocal" "0, 0, 0")
      (Actor|DestroyActor))
    (:CastFailed
      (Audio|PlaySoundatLocation "/Game/Audio/SC_Ground_Magic_Hit.SC_Ground_Magic_Hit" _impactpoint "0, 0, 0" 1.0 1.0 0.0 0 0 0 0)
      (Niagara|SpawnSystematLocation "/Game/VFX/NS_Demon_Impact.NS_Demon_Impact" _impactpoint)
      (Actor|DestroyActor))))

(event OnComponentBeginOverlap(Sphere)
  (params (OverlappedComponent :type Primitive%20Component%20Object%20Reference) (OtherActor :type Actor%20Object%20Reference) (OtherComp :type Primitive%20Component%20Object%20Reference) (OtherBodyIndex :type Integer) (bFromSweep :type Boolean) (SweepResult :type Hit%20Result%20Structure%20%28by%20ref%29))
  (bind _impactpoint (Collision|BreakHitResult SweepResult))
  (Utilities|Casting|CastToBP_FirstPersonCharacter OtherActor
    (:then
      (Audio|PlaySoundatLocation "/Game/Audio/SC_Bat_Hit.SC_Bat_Hit" _impactpoint "0, 0, 0" 1.0 1.0 0.0 0 0 0 0)
      (Niagara|SpawnSystematLocation "/Game/VFX/NS_Demon_Impact.NS_Demon_Impact" _impactpoint)
      (Class|LegacyCameraShake|StartLegacyCameraShake (Game|GetPlayerCameraManager 0) "/Game/Blueprints/BP_Take_Damage_Screen_Shake.BP_Take_Damage_Screen_Shake_C" 1.0 "CameraLocal" "0, 0, 0")
      (Actor|DestroyActor))
    (:CastFailed
      (Audio|PlaySoundatLocation "/Game/Audio/SC_Ground_Magic_Hit.SC_Ground_Magic_Hit" _impactpoint "0, 0, 0" 1.0 1.0 0.0 0 0 0 0)
      (Niagara|SpawnSystematLocation "/Game/VFX/NS_Demon_Impact.NS_Demon_Impact" _impactpoint)
      (Actor|DestroyActor))))

(event EventBeginPlay
  (bind _scale (Timeline|Timeline_0 PlayFromStart)
    (:Update
      (Transformation|SetRelativeScale3D (Variables|Default|GetSphere) _scale))))

(event EventTick
  (params (DeltaSeconds :type Float%20%28single-precision%29))
  (Variables|/Script/Engine.ProjectileMovementComponent|SetHomingTargetComponent (Variables|Default|GetProjectileMovement) (Variables|/Script/Engine.Character|GetCapsuleComponent (Game|GetPlayerCharacter 0))))

(fn ConstructionScript)